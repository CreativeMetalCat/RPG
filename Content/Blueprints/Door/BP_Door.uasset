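; BP_Door is an interactable door that toggles between open and closed.
; It swaps visibility between the DoorClosed and DoorOpen components rather than animating, with the construction script applying the initial Open state.
; Interact flips the state, plays a sound at the door's location and toggles ShadowMesh shadow casting, with InverseOpen reversing that shadow logic.
; DealDamage is a stub that returns zero.
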(event EventBeginPlay)

(event Collision|EventActorBeginOverlap
  (params (OtherActor :type Actor%20Object%20Reference)))

(event EventTick
  (params (DeltaSeconds :type Float%20%28single-precision%29)))

(event EventInteract
  (params (Interactor :type Actor%20Object%20Reference))
  (Variables|Default|SetOpen (not (Variables|Default|GetOpen)))
  (Rendering|SetVisibility (Variables|Default|GetDoorClosed) (not (Variables|Default|GetOpen)) false)
  (Rendering|SetVisibility (Variables|Default|GetDoorOpen) (Variables|Default|GetOpen) false)
  (Audio|PlaySoundatLocation (Variables|Default|GetDoorInteractionSound) (Transformation|GetActorLocation) "0, 0, 0" 1.0 1.0 0.0 0 0 0)
  (Rendering|SetCastShadow (Variables|Default|GetShadowMesh) (select (Variables|Default|GetInverseOpen) (Variables|Default|GetOpen) (not (Variables|Default|GetOpen)))))

(fn ConstructionScript
  (bind _open (Variables|Default|GetOpen))
  (Rendering|SetVisibility (Variables|Default|GetDoorClosed) (not _open) false)
  (Rendering|SetVisibility (Variables|Default|GetDoorOpen) _open false))

(fn DealDamage
  (params (Damage :type Integer) (DamageDealer :type Actor%20Object%20Reference) (SpecialEffect :type Special%20Effect%20Class%20Reference))
  (return 0))
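; Tilemap actor that hides its ceiling layers while something overlaps its render component.
; Overlap begin and end subtract and add 1 to the alpha of each layer in CeilingLayersIds, without filtering the overlapping actor.
; The layer change requires a tilemap converted to an instance, otherwise an error prints.
; The construction script applies a translucent lit or unlit sprite material based on the Lit flag.
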(event OnComponentBeginOverlap(RenderComponent)
  (params (OverlappedComponent :type Primitive%20Component%20Object%20Reference) (OtherActor :type Actor%20Object%20Reference) (OtherComp :type Primitive%20Component%20Object%20Reference) (OtherBodyIndex :type Integer) (bFromSweep :type Boolean) (SweepResult :type Hit%20Result%20Structure%20%28by%20ref%29))
  (bind _rendercomponent (Variables|Default|GetRenderComponent))
  (if (Class|PaperTileMapComponent|OwnsTileMap (Variables|Default|GetRenderComponent))
    (for _array_element (Variables|Default|GetCeilingLayersIds)
      (Class|PaperTileMapComponent|SetLayerColor _rendercomponent (Math|Color|MakeColor (.R (Math|Color|BreakColor (Class|PaperTileMapComponent|GetLayerColor _rendercomponent _array_element))) (.G (Math|Color|BreakColor (Class|PaperTileMapComponent|GetLayerColor _rendercomponent _array_element))) (.B (Math|Color|BreakColor (Class|PaperTileMapComponent|GetLayerColor _rendercomponent _array_element))) (- (.A (Math|Color|BreakColor (Class|PaperTileMapComponent|GetLayerColor _rendercomponent _array_element))) 1.0)) _array_element))
    (else
      (Development|PrintString (Utilities|String|Append "Error: " (Utilities|GetObjectName self) " Attempts to change visibilty of tilemap layers, but tilemap wasn't converted to instance!") true true "(R=1.000000,G=0.000000,B=0.000000,A=1.000000)"))))

(event OnComponentEndOverlap(RenderComponent)
  (params (OverlappedComponent :type Primitive%20Component%20Object%20Reference) (OtherActor :type Actor%20Object%20Reference) (OtherComp :type Primitive%20Component%20Object%20Reference) (OtherBodyIndex :type Integer))
  (bind _rendercomponent (Variables|Default|GetRenderComponent))
  (if (Class|PaperTileMapComponent|OwnsTileMap (Variables|Default|GetRenderComponent))
    (for _array_element (Variables|Default|GetCeilingLayersIds)
      (Class|PaperTileMapComponent|SetLayerColor _rendercomponent (Math|Color|MakeColor (.R (Math|Color|BreakColor (Class|PaperTileMapComponent|GetLayerColor _rendercomponent _array_element))) (.G (Math|Color|BreakColor (Class|PaperTileMapComponent|GetLayerColor _rendercomponent _array_element))) (.B (Math|Color|BreakColor (Class|PaperTileMapComponent|GetLayerColor _rendercomponent _array_element))) (- (.A (Math|Color|BreakColor (Class|PaperTileMapComponent|GetLayerColor _rendercomponent _array_element))) -1.0)) _array_element))
    (else
      (Development|PrintString (Utilities|String|Append "Error: " (Utilities|GetObjectName self) " Attempts to change visibilty of tilemap layers, but tilemap wasn't converted to instance!") true true "(R=1.000000,G=0.000000,B=0.000000,A=1.000000)"))))

(event EventBeginPlay)

(event Collision|EventActorBeginOverlap
  (params (OtherActor :type Actor%20Object%20Reference)))

(event EventTick
  (params (DeltaSeconds :type Float%20%28single-precision%29)))

(fn ConstructionScript
  (bind _rendercomponent (Variables|Default|GetRenderComponent))
  (if (Variables|Default|GetLit)
    (Rendering|Material|SetMaterial _rendercomponent 0 "/Paper2D/TranslucentLitSpriteMaterial.TranslucentLitSpriteMaterial")
    (else
      (Rendering|Material|SetMaterial _rendercomponent 0 "/Paper2D/TranslucentUnlitSpriteMaterial.TranslucentUnlitSpriteMaterial"))))
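; BP_MovableObject is an object that RPG characters push along one of four axis-aligned directions.
; Four side detection volumes record the pusher and opposite direction, then start a delay timer.
; When it fires, movement begins only if the pusher still overlaps that side and faces the push direction.
; Tick eases the offset from the start location toward a set distance, and any Collision overlap halts it.
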(event OnComponentBeginOverlap(Collision)
  (params (OverlappedComponent :type Primitive%20Component%20Object%20Reference) (OtherActor :type Actor%20Object%20Reference) (OtherComp :type Primitive%20Component%20Object%20Reference) (OtherBodyIndex :type Integer) (bFromSweep :type Boolean) (SweepResult :type Hit%20Result%20Structure%20%28by%20ref%29))
  ;[1 1 1] Stop movement
  (Variables|Movement|SetShouldMove false)
  (Variables|Movement|SetCurrentMovementAmount 0.0))

(event OnComponentBeginOverlap(DetectionUp)
  (params (OverlappedComponent :type Primitive%20Component%20Object%20Reference) (OtherActor :type Actor%20Object%20Reference) (OtherComp :type Primitive%20Component%20Object%20Reference) (OtherBodyIndex :type Integer) (bFromSweep :type Boolean) (SweepResult :type Hit%20Result%20Structure%20%28by%20ref%29))
  ;[1 1 1] Start check
  (CallFunction|StartPushing (delegate Custom|Move) OtherActor "ED_Down"))

(event OnComponentBeginOverlap(DetectionDown)
  (params (OverlappedComponent :type Primitive%20Component%20Object%20Reference) (OtherActor :type Actor%20Object%20Reference) (OtherComp :type Primitive%20Component%20Object%20Reference) (OtherBodyIndex :type Integer) (bFromSweep :type Boolean) (SweepResult :type Hit%20Result%20Structure%20%28by%20ref%29))
  ;[1 1 1] Start check
  (CallFunction|StartPushing (delegate Custom|Move) OtherActor "ED_Up"))

(event OnComponentBeginOverlap(DetectionLeft)
  (params (OverlappedComponent :type Primitive%20Component%20Object%20Reference) (OtherActor :type Actor%20Object%20Reference) (OtherComp :type Primitive%20Component%20Object%20Reference) (OtherBodyIndex :type Integer) (bFromSweep :type Boolean) (SweepResult :type Hit%20Result%20Structure%20%28by%20ref%29))
  ;[1 1 1] Start check
  (CallFunction|StartPushing (delegate Custom|Move) OtherActor "ED_Right"))

(event OnComponentBeginOverlap(DetectionRight)
  (params (OverlappedComponent :type Primitive%20Component%20Object%20Reference) (OtherActor :type Actor%20Object%20Reference) (OtherComp :type Primitive%20Component%20Object%20Reference) (OtherBodyIndex :type Integer) (bFromSweep :type Boolean) (SweepResult :type Hit%20Result%20Structure%20%28by%20ref%29))
  ;[1 1 1] Start check
  (CallFunction|StartPushing (delegate Custom|Move) OtherActor "ED_Left"))

(event Custom|Move
  (if (CallFunction|IsStillPushing)
    (Variables|Default|SetLocationAtTheStart (Transformation|GetActorLocation))
    (Variables|Movement|SetShouldMove true)))

(event EventTick
  (params (DeltaSeconds :type Float%20%28single-precision%29))
  (bind _locationatthestart (Variables|Default|GetLocationAtTheStart))
  (bind _locationatthestart_2 (Variables|Default|GetLocationAtTheStart))
  (bind _locationatthestart_3 (Variables|Default|GetLocationAtTheStart))
  (bind _movementamount (Variables|Movement|GetMovementAmount))
  (bind _locationatthestart_4 (Variables|Default|GetLocationAtTheStart))
  (bind (_x _y _z) (Math|Vector|BreakVector _locationatthestart_4))
  (bind (_x_2 _y_2 _z_2) (Math|Vector|BreakVector _locationatthestart))
  (bind (_x_3 _y_3 _z_3) (Math|Vector|BreakVector _locationatthestart_2))
  (bind (_x_4 _y_4 _z_4) (Math|Vector|BreakVector _locationatthestart_3))
  ;[1 1 1] Update
  (if (Variables|Movement|GetShouldMove)
    (bind _output_get (Variables|Movement|SetCurrentMovementAmount (Math|Interpolation|FInterpTo (Variables|Movement|GetCurrentMovementAmount) _movementamount DeltaSeconds (Variables|Movement|GetMovementSpeed))))
    (if (>= _output_get _movementamount)
      (Variables|Movement|SetShouldMove false))
    (switch Utilities|FlowControl|Switch|SwitchonEDirection (Variables|Movement|GetDesiredMovementDirection)
      (:ED_Up
        (Transformation|SetActorLocation (Math|Vector|MakeVector _x_2 (- _y_2 _output_get) _z_2) false false))
      (:ED_Down
        (Transformation|SetActorLocation (Math|Vector|MakeVector _x_3 (+ _y_3 _output_get) _z_3) false false))
      (:ED_Right
        (Transformation|SetActorLocation (Math|Vector|MakeVector (+ _x_4 _output_get) _y_4 _z_4) false false))
      (:ED_Left
        (Transformation|SetActorLocation (Math|Vector|MakeVector (- _x _output_get) _y _z) false false)))))

(fn ConstructionScript)

(fn IsStillPushing
  (bind _pusher (Variables|Push|GetPusher))
  (return (and (!= (Utilities|Array|FindItem (Collision|GetOverlappingActors (Utilities|Select :Index (Variables|Movement|GetDesiredMovementDirection) :ED_Up (Variables|Default|GetDetectionDown) :ED_Down (Variables|Default|GetDetectionUp) :ED_Right (Variables|Default|GetDetectionLeft) :ED_Left (Variables|Default|GetDetectionRight)) "/Script/RPGCore.RPGCharacterBase" :!class /Script/Engine.PrimitiveComponent) _pusher) -1) (Utilities|Enum|Equal(Enum) (Variables|/Script/RPGCore.RPGCharacterBase|GetCurrentDirection _pusher) (Variables|Movement|GetDesiredMovementDirection)))))

(fn StartPushing
  (params (Delegate :type Delegate) (Actor :type Actor%20Object%20Reference) (DesiredDirection :type EDirection%20Enum :default "ED_Up"))
  (if (not (Variables|Movement|GetShouldMove))
    (Variables|Movement|SetCurrentMovementAmount 0.0)
    (bind _asrpgcharacter_base (Utilities|Casting|CastToRPGCharacterBase Actor))
    (Variables|Push|SetPusher _asrpgcharacter_base)
    (Variables|Movement|SetDesiredMovementDirection DesiredDirection)
    (Utilities|Time|SetTimerbyEvent Delegate (Variables|Push|GetTimeToPush))))

(fn ComponentstoSave
  (return 0))
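; BP_Bush is a destructible bush object drawn with a Paper2D flipbook.
; DealDamage subtracts damage from Health, calls Break when the result is zero or less, and returns that result without storing it in Health.
; Break plays the destroyed flipbook once and removes the shadow and collision components, leaving the actor in place.
; Its event graph and construction script have no active logic.
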(event EventBeginPlay)

(event Collision|EventActorBeginOverlap
  (params (OtherActor :type Actor%20Object%20Reference)))

(event EventTick
  (params (DeltaSeconds :type Float%20%28single-precision%29)))

(fn ConstructionScript)

(fn Break
  (bind _paperflipbook (Variables|Default|GetPaperFlipbook))
  (Sprite|SetFlipbook _paperflipbook "/Game/Assets/Sprites/Bush/FB_Bush_Destroyed.FB_Bush_Destroyed")
  (Components|Timeline|SetLooping _paperflipbook false)
  (Audio|Components|Audio|Play _paperflipbook)
  (Components|DestroyComponent (Variables|Default|GetShadow)))

(fn DealDamage
  (params (Damage :type Integer) (DamageDealer :type Actor%20Object%20Reference) (SpecialEffect :type Special%20Effect%20Class%20Reference))
  (bind _health (Variables|Default|GetHealth))
  (bind _returnvalue (- _health Damage))
  (if (<= _returnvalue 0)
    (CallFunction|Break))
  (return _returnvalue))
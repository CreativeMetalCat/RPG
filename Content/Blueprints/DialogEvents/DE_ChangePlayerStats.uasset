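; DE_ChangePlayerStats is a dialog event that changes the player's health, attack power and magic juice.
; When triggered, it casts the considering player's controlled pawn to BP_Player and stops if that fails.
; An AddToExisting flag chooses between adding to all three stats and overwriting them.
; Additions to health and magic juice go through the player's Add functions, while attack power and all overwrites set variables directly.
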(event EventRecieveEventTriggered
  (params (ConsideringPlayer :type Player%20Controller%20Object%20Reference) (NPCActor :type Actor%20Object%20Reference))
  (bind _addtoexisting_ (Variables|Default|GetAddToExisting?))
  (bind _attack (Variables|Default|GetAttack))
  (bind _magicjuice (Variables|Default|GetMagicJuice))
  (bind _asbp_player (Utilities|Casting|CastToBP_Player (Pawn|GetControlledPawn ConsideringPlayer)))
  (if _addtoexisting_
    (Class|RPGCharacterBase|AddHealth _asbp_player (Variables|Default|GetHealth))
    (else
      (Variables|/Script/RPGCore.RPGCharacterBase|SetHealth _asbp_player (Variables|Default|GetHealth))))
  (Variables|/Script/RPGCore.RPGCharacterBase|SetAttackPower _asbp_player (select _addtoexisting_ (+ (Variables|/Script/RPGCore.RPGCharacterBase|GetAttackPower _asbp_player) _attack) _attack))
  (if _addtoexisting_
    (Class|RPGCharacterBase|AddMagicJuice _asbp_player _magicjuice)
    (else
      (Variables|/Script/RPGCore.RPGCharacterBase|SetCurrentMagicJuice _asbp_player _magicjuice))))
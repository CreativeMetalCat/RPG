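; Dialog event that takes a required item from the player and advances a quest in exchange.
; When triggered, it resolves the needed item's data table row and checks that the controlled BP_Player holds enough of it.
; If removal succeeds, it looks up the quest row and calls MakeProgress on the player with the configured amount.
; Any failed cast, lookup, check or removal ends the event without quest progress.
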(event EventRecieveEventTriggered
  (params (ConsideringPlayer :type Player%20Controller%20Object%20Reference) (NPCActor :type Actor%20Object%20Reference))
  (bind _quest (Variables|Default|GetQuest))
  (bind _neededitem (Variables|Default|GetNeededItem))
  (bind _neededitemamout (Variables|Default|GetNeededItemAmout))
  (bind (_datatable _rowname) (Utilities|Struct|BreakDataTableRowHandle _quest))
  (bind (_datatable_2 _rowname_2) (Utilities|Struct|BreakDataTableRowHandle _neededitem))
  (bind _asbp_player (Utilities|Casting|CastToBP_Player (Pawn|GetControlledPawn ConsideringPlayer)))
  (bind _returnvalue (Utilities|GetDataTableRow _datatable_2 _rowname_2)
    (:then
      (if (.hasItem (Class|RPGCharacterBase|GetItembyName _asbp_player (.DevName (Utilities|Struct|BreakItemInfo _returnvalue))))
        (if (>= (Utilities|Struct|BreakItemInfo (.ReturnValue (Class|RPGCharacterBase|GetItembyName _asbp_player (.DevName (Utilities|Struct|BreakItemInfo _returnvalue))))) _neededitemamout)
          (bind _returnvalue_2 (Class|RPGCharacterBase|RemoveItem _asbp_player (.DevName (Utilities|Struct|BreakItemInfo _returnvalue)) _neededitemamout))
          (if _returnvalue_2
            (bind _returnvalue_3 (Utilities|GetDataTableRow _datatable _rowname)
              (:then
                (Class|PlayerBase|MakeProgress _asbp_player (.DevName (Utilities|Struct|BreakQuestInfo _returnvalue_3)) (Variables|Default|GetAmountOfProgress))))))))))
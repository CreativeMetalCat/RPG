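; Paper2D spike trap puzzle element that periodically extends and retracts, damaging actors in its damage area while active.
; Switch flips the state, reschedules itself with separate active and inactive durations, and starts or clears a looping damage timer that messages overlapping actors.
; One activation flipbook plays forward or reversed for transitions, then gives way to visible or hidden idle flipbooks.
; ToggleMechanism flips IsWorking and halts the cycle when off, without restarting it when on.
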(event OnFinishedPlaying(PaperFlipbook)
  ;[1 1 1] Set flipbook
  (Sprite|SetFlipbook (Variables|Default|GetPaperFlipbook) (select (Variables|AutoToggle|GetActive) (Variables|Flipbooks|GetVisibleSpikesFlipbook) (Variables|Flipbooks|GetHiddenSpikesFlipbook))))

(event Custom|Switch
  (bind _activatonflipbook (Variables|Flipbooks|GetActivatonFlipbook))
  (bind _paperflipbook (Variables|Default|GetPaperFlipbook))
  (if (Variables|Default|GetIsWorking)
    (Variables|AutoToggle|SetActive (not (Variables|AutoToggle|GetActive)))
    ;[1 1 1] Update sprites
    (Sprite|SetFlipbook _paperflipbook _activatonflipbook)
    (Components|Timeline|SetPlayRate _paperflipbook (Math|Float|SelectFloat 1.0 -1.0 (Variables|AutoToggle|GetActive)))
    (Components|Timeline|SetLooping _paperflipbook false)
    (Components|Timeline|SetPlaybackPosition _paperflipbook (Math|Float|SelectFloat 0.0 (Class|PaperFlipbook|GetTotalDuration _activatonflipbook) (Variables|AutoToggle|GetActive)) false)
    (Audio|Components|Audio|Play _paperflipbook)
    (bind _returnvalue (Utilities|Time|SetTimerbyEvent (delegate Custom|Switch) (Math|Float|SelectFloat (Variables|AutoToggle|GetActiveTime) (Variables|AutoToggle|GetInActiveTime) (Variables|AutoToggle|GetActive))))
    (Variables|AutoToggle|SetSwitchTimer _returnvalue)
    (if (Variables|AutoToggle|GetActive)
      (bind _returnvalue_2 (Utilities|Time|SetTimerbyEvent (delegate Custom|DealDamageToOverlaped) (Variables|Damage|GetDamageInterval) true))
      (Variables|Damage|Timer|SetDamageTimerHandle _returnvalue_2)
      (else
        (Utilities|Time|ClearandInvalidateTimerbyHandle (Variables|Damage|Timer|GetDamageTimerHandle))))))

(event Custom|DealDamageToOverlaped
  ;[1 1 1] Deal damage
  (Development|PrintString "DAMAGE" true false)
  (for _array_element (Collision|GetOverlappingActors (Variables|Default|GetDamageArea) "/Script/Engine.Actor" :!class /Script/Engine.PrimitiveComponent)
    (Utilities|IsValid _array_element
      (:Is%20Valid
        (Class|Interaction|DealDamage(Message) _array_element (Variables|Damage|GetDamage) self (Variables|Damage|GetDamageEffects))))))

(event EventBeginPlay
  ;[1 1 1] Begin play
  (if (Variables|Default|GetIsWorking)
    (CallFunction|Switch)
    (elif (Variables|AutoToggle|GetActive)
      (bind _returnvalue (Utilities|Time|SetTimerbyEvent (delegate Custom|DealDamageToOverlaped) (Variables|Damage|GetDamageInterval) true))
      (Variables|Damage|Timer|SetDamageTimerHandle _returnvalue)
      (else
        (Utilities|Time|ClearandInvalidateTimerbyHandle (Variables|Damage|Timer|GetDamageTimerHandle))))))

(event EventToggleMechanism
  (params (activator :type Actor%20Object%20Reference))
  (bind _output_get (Variables|Default|SetIsWorking (not (Variables|Default|GetIsWorking))))
  (if (not _output_get)
    (Utilities|Time|ClearandInvalidateTimerbyHandle (Variables|AutoToggle|GetSwitchTimer))))

(fn ConstructionScript
  (bind _visiblespikesflipbook (Variables|Flipbooks|GetVisibleSpikesFlipbook))
  (bind _hiddenspikesflipbook (Variables|Flipbooks|GetHiddenSpikesFlipbook))
  (Utilities|IsValid _visiblespikesflipbook
    (:Is%20Valid
      (Utilities|IsValid _hiddenspikesflipbook
        (:Is%20Valid
          (Sprite|SetFlipbook (Variables|Default|GetPaperFlipbook) (select (Variables|AutoToggle|GetActive) _hiddenspikesflipbook _visiblespikesflipbook)))))))

(fn DealDamage
  (params (Damage :type Integer) (DamageDealer :type Actor%20Object%20Reference) (SpecialEffect :type Special%20Effect%20Class%20Reference))
  (return 0))
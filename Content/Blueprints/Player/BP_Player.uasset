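; Player character Blueprint that layers HUD, input and sound feedback over inherited stats, quest, item, ability and combat logic.
; BeginPlay grants editor-only start items, creates the HUD and registers quests from DT_Quest.
; Overrides call the parent, most then refreshing the HUD or playing level-up and death feedback.
; Input drives an ability, shield, pause menu and bug report, plus apparent debug keys that adjust max health.
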(event Custom|CustomEvent
  (bind _hud (Variables|Default|GetHUD)
    (:then
      (Default|UpdateQuestInfo _hud))
    (:else)))

(event Custom|CustomEvent_1
  (bind _hud (Variables|Default|GetHUD)
    (:then
      (Default|UpdatePlayerInfo _hud))
    (:else)))

(event EventBeginPlay
  ;[0.6577 1 0] Give items to player(Editor only)
  (if (not (Class|KismetSystemLibrary|IsPackagedforDistribution))
    (for _array_element (Variables|Default|GetStartItems)
      (bind _returnvalue (Utilities|GetDataTableRow (.DataTable (Utilities|Struct|BreakDataTableRowHandle _array_element)) (.RowName (Utilities|Struct|BreakDataTableRowHandle _array_element)))
        (:then
          (CallFunction|AddItem _returnvalue))
        (:RowNotFound
          ;[0.1563 1 0.1972] Create HUD
          (bind _returnvalue_2 (UserInterface|CreateWidget "/Game/Blueprints/UI/UMG_HUD.UMG_HUD_C" 0 self))
          (bind _output_get (Variables|Default|SetHUD _returnvalue_2))
          (UserInterface|Viewport|AddtoViewport _output_get 0)
          ;[0.3991 0.436 1] This adds every quest that player doesn't have
          (bind _outrownames (DataTable|GetDataTableRowNames "/Game/DataTables/DT_Quest.DT_Quest"))
          (for _array_element_2 _outrownames
            (bind _returnvalue_3 (Utilities|GetDataTableRow "/Game/DataTables/DT_Quest.DT_Quest" _array_element_2)
              (:then
                (Class|PlayerBase|AddQuesttoQuestArray _returnvalue_3) ; This way if player has quest completed it won't be overriden
              )))))))
  (bind _returnvalue_4 (UserInterface|CreateWidget "/Game/Blueprints/UI/UMG_HUD.UMG_HUD_C" 0 self))
  (bind _output_get_2 (Variables|Default|SetHUD _returnvalue_4))
  (UserInterface|Viewport|AddtoViewport _output_get_2 0)
  (bind _outrownames_2 (DataTable|GetDataTableRowNames "/Game/DataTables/DT_Quest.DT_Quest"))
  (for _array_element_3 _outrownames_2
    (bind _returnvalue_5 (Utilities|GetDataTableRow "/Game/DataTables/DT_Quest.DT_Quest" _array_element_3)
      (:then
        (Class|PlayerBase|AddQuesttoQuestArray _returnvalue_5) ; This way if player has quest completed it won't be overriden
      ))))

(event Collision|EventActorBeginOverlap
  (params (OtherActor :type Actor%20Object%20Reference)))

(event EventTick
  (params (DeltaSeconds :type Float%20%28single-precision%29))
  ;[1 0 0] DEVELOPMENT ONLY
  (Transformation|SetRelativeRotation (Variables|Default|GetArrow1) (Utilities|Select :Index (Variables|Default|GetCurrentDirection) :Option%200 "0, 0, 0" :Option%201 "0, 0, 0" :Option%202 "0, 0, 0" :Option%203 "0, 0, 0") false false))

(event EventDie
  (if (not (Variables|Default|GetbDead))
    (|CallParentFunction)
    (Audio|PlaySound2D "/Game/Assets/Retro_8Bit_Sounds/Retro_Orginal/Wavs/retro_fail_sound_04.retro_fail_sound_04" 1.0 1.0 0.0 0 0)
    (Utilities|PlayAnimation "/Game/Assets/Sprites/Character/temp/Anims/Die/PlaceHolderCharacterDie1.PlaceHolderCharacterDie1")))

(event EventLevelUp
  (|CallParentFunction)
  (Audio|PlaySound2D "/Game/Assets/Retro_8Bit_Sounds/Music/Wavs/retro__musical_stinger_02.retro__musical_stinger_02" 1.0 1.0 0.0 0 0)
  (bind _hud (Variables|Default|GetHUD)
    (:then
      (Default|UpdatePlayerInfo _hud))
    (:else)))

(event EventUpdatePlayerInfo
  ;[1 1 1] Update player info
  (bind _hud (Variables|Default|GetHUD)
    (:then
      (Default|UpdatePlayerInfo _hud)
      (Default|UpdateQuestInfo _hud))
    (:else)))

(event EventMakeProgress
  (params (devName :type String) (amount :type Integer))
  (|CallParentFunction devName amount)
  (bind _hud (Variables|Default|GetHUD)
    (:then
      (Default|UpdateQuestInfo _hud))
    (:else)))

(event Input|ActionEvents|InputActionHoldShield
  (params (Key :type Key%20Structure :default "None"))
  ;[1 1 1] Hold Shield
  (:Pressed
    (Class|RPGCharacterBase|PutUpShield))
  (:Released
    (Class|RPGCharacterBase|PutDownShield)))

(event Input|ActionEvents|InputActionPause
  (params (Key :type Key%20Structure :default "None"))
  ;[1 1 1] Pause
  (:Pressed
    (bind _returnvalue (UserInterface|CreateWidget "/Game/Blueprints/UI/Menu/UMG_Menu.UMG_Menu_C" 0 true))
    (UserInterface|Viewport|AddtoViewport _returnvalue 0)))

(event Input|KeyboardEvents|1
  (params (Key :type Key%20Structure :default "None"))
  (:Pressed
    (if (.has (Class|RPGCharacterBase|GetAbilityInfo))
      (Class|RPGCharacterBase|UseAbility))))

(event Input|KeyboardEvents|F8
  (params (Key :type Key%20Structure :default "None"))
  ;[1 1 1] Bug Report
  (:Pressed
    (bind _returnvalue (UserInterface|CreateWidget "/Game/Blueprints/DiscordBugReport/UMG_BugReport.UMG_BugReport_C"))
    (UserInterface|Viewport|AddtoViewport _returnvalue 0)))

(event Input|KeyboardEvents|Add
  (params (Key :type Key%20Structure :default "None"))
  (:Pressed
    (Variables|Default|SetMaxHealth (+ (Variables|Default|GetMaxHealth) 10))
    (Class|RPGCharacterBase|UpdatePlayerInfo)))

(event Input|KeyboardEvents|Subtract
  (params (Key :type Key%20Structure :default "None"))
  (:Pressed
    (Variables|Default|SetMaxHealth (+ (Variables|Default|GetMaxHealth) -10))
    (Class|RPGCharacterBase|UpdatePlayerInfo)))

(fn ConstructionScript)

(fn AddAbilityfromTable
  (params (DevName :type String))
  (bind _returnvalue (Utilities|GetDataTableRow "/Game/DataTables/DT_Abilitiy.DT_Abilitiy" (Utilities|String|StringToName DevName))
    (:then
      (bind _returnvalue_2 (Class|RPGCharacterBase|AddAbility _returnvalue))
      (return _returnvalue_2))
    (:RowNotFound
      (return false))))

(fn AddQuest
  (params (quest :type Quest%20Info%20Structure))
  (bind _returnvalue (|CallParentFunction quest))
  (bind _hud (Variables|Default|GetHUD)
    (:then
      (Default|UpdateQuestInfo _hud))
    (:else
      _))
  (return _returnvalue))

(fn CompleteQuest
  (params (devName :type String) (questId :type Integer))
  (bind _returnvalue (|CallParentFunction devName questId))
  (bind _hud (Variables|Default|GetHUD)
    (:then
      (Default|UpdateQuestInfo _hud))
    (:else
      _))
  (return _returnvalue))

(fn DealDamage
  (params (Damage :type Integer) (DamageDealer :type Actor%20Object%20Reference) (SpecialEffect :type Special%20Effect%20Class%20Reference))
  (bind _returnvalue (|CallParentFunction Damage DamageDealer SpecialEffect))
  (return _returnvalue))

(fn AddItem
  (params (item :type Item%20Info%20Structure))
  (bind _returnvalue (|CallParentFunction item))
  (Development|PrintString (.DevName (Utilities|Struct|BreakItemInfo item)))
  (return _returnvalue))

(fn ComponentstoSave
  (return 0))
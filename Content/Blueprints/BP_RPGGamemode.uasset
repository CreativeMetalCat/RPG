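; RPG game mode that restores saved progress when play starts, moving the player to the last saved level.
; BeginPlay sets a hardcoded temporary save slot, then opens the profile's saved level if it differs from the current one.
; Otherwise it polls until the restarted player is valid, async-loads saved actors when levels match, then fires OnLoaded and clears ShouldLoadGame.
; OnRestartPlayer enters the same wait-and-load path.
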(event EventBeginPlay
  (bind _returnvalue (Class|EMSFunctionLibrary|GetLocalProfileSaveGame))
  (bind _asbp_save_profile (Utilities|Casting|CastToBP_SaveProfile _returnvalue))
  (bind _lastsavedlevelname (Variables|/Game/Blueprints/SaveSystem/BP_SaveProfile.BP_SaveProfile_C|GetLastSavedLevelName _asbp_save_profile))
  ;[1 0 0] TODO: Remove this
  (Class|EMSFunctionLibrary|SetCurrentSaveUserName "SaveSlot1")
  ;[1 1 1] Load level if spawned in wrong one
  (bind _returnvalue_2 (Game|GetCurrentLevelName true))
  (if (and (Utilities|Enum|NotEqual(Enum) _returnvalue_2 _lastsavedlevelname) (Utilities|Enum|NotEqual(Enum) _lastsavedlevelname ""))
    (Variables|/Game/Blueprints/BP_GameInstance.BP_GameInstance_C|SetLoadLevel (.AsBP%20Game%20Instance (Utilities|Casting|CastToBP_GameInstance (Game|GetGameInstance))) false)
    (Game|OpenLevel(byName) (Utilities|String|StringToName _lastsavedlevelname))
    (else
      ;[1 1 1] Stupid but works - Wait untill unreal creates player and then load
      (Utilities|IsValid (stale EventOnRestartPlayer NewPlayer) :!label _label
        (:Is%20Valid
          (Class|EMSFunctionLibrary|SetCurrentSaveGameName (Variables|/Game/Blueprints/SaveSystem/BP_SaveProfile.BP_SaveProfile_C|GetLastSavedLevelName (.AsBP%20Save%20Profile (Utilities|Casting|CastToBP_SaveProfile (Class|EMSFunctionLibrary|GetLocalProfileSaveGame)))))
          (bind _returnvalue_3 (Game|GetCurrentLevelName true))
          (if (Utilities|Enum|Equal(Enum) (Variables|/Game/Blueprints/SaveSystem/BP_SaveProfile.BP_SaveProfile_C|GetLastSavedLevelName (.AsBP%20Save%20Profile (Utilities|Casting|CastToBP_SaveProfile (Class|EMSFunctionLibrary|GetLocalProfileSaveGame)))) _returnvalue_3)
            (|AsyncLoadActors 3 true
              (:OnCompleted
                (CallFunction|OnLoaded)
                (bind _asbp_persistent_save (Utilities|Casting|CastToBP_PersistentSave (Class|EMSFunctionLibrary|GetPersistentSave)))
                (Variables|/Game/Blueprints/SaveSystem/BP_PersistentSave.BP_PersistentSave_C|SetShouldLoadGame _asbp_persistent_save false)))))
        (:Is%20Not%20Valid
          (Utilities|FlowControl|Delay 0.1)
          (goto _label))))))

(event EventTick
  (params (DeltaSeconds :type Float%20%28single-precision%29)))

(event EventOnRestartPlayer
  (params (NewPlayer :type Controller%20Object%20Reference))
  ;[1 1 1] Stupid but works - Wait untill unreal creates player and then load
  (Utilities|IsValid NewPlayer :!label _label
    (:Is%20Valid
      (Class|EMSFunctionLibrary|SetCurrentSaveGameName (Variables|/Game/Blueprints/SaveSystem/BP_SaveProfile.BP_SaveProfile_C|GetLastSavedLevelName (.AsBP%20Save%20Profile (Utilities|Casting|CastToBP_SaveProfile (Class|EMSFunctionLibrary|GetLocalProfileSaveGame)))))
      (bind _returnvalue (Game|GetCurrentLevelName true))
      (if (Utilities|Enum|Equal(Enum) (Variables|/Game/Blueprints/SaveSystem/BP_SaveProfile.BP_SaveProfile_C|GetLastSavedLevelName (.AsBP%20Save%20Profile (Utilities|Casting|CastToBP_SaveProfile (Class|EMSFunctionLibrary|GetLocalProfileSaveGame)))) _returnvalue)
        (|AsyncLoadActors 3 true
          (:OnCompleted
            (CallFunction|OnLoaded)
            (bind _asbp_persistent_save (Utilities|Casting|CastToBP_PersistentSave (Class|EMSFunctionLibrary|GetPersistentSave)))
            (Variables|/Game/Blueprints/SaveSystem/BP_PersistentSave.BP_PersistentSave_C|SetShouldLoadGame _asbp_persistent_save false)))))
    (:Is%20Not%20Valid
      (Utilities|FlowControl|Delay 0.1)
      (goto _label))))

(fn ConstructionScript)
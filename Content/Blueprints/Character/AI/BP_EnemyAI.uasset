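; BP_EnemyAI is the enemy AI controller, which hands decision-making to the BT_BasicEnemy behavior tree.
; On BeginPlay it calls the parent and starts the tree only if the controlled pawn casts to EnemyCharacterBase.
; Tick is empty, and the MovementType check, MoveTo call and goal debug print are disconnected leftovers that never run.
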(event EventBeginPlay
  (|CallParentFunction)
  (if (.bSuccess (Utilities|Casting|CastToEnemyCharacterBase (Pawn|GetControlledPawn)))
    (AI|RunBehaviorTree "/Game/Blueprints/Character/AI/BT_BasicEnemy.BT_BasicEnemy")))

(event EventTick
  (params (DeltaSeconds :type Float%20%28single-precision%29)))

(fn ConstructionScript)
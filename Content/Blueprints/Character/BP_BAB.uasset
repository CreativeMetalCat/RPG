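; BP_BAB is a character, apparently a placeholder bad guy, that can take damage, die and open dialog when the player interacts.
; Death plays sound and animation, then fakes destruction for the SaveSystem by hiding and disabling the actor, unpossessing its controller and clearing applied effects.
; ActorLoaded reapplies that disabled state if Dead is set.
; DealDamage calls the parent implementation and prints a debug message.
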(event EventBeginPlay)

(event Collision|EventActorBeginOverlap
  (params (OtherActor :type Actor%20Object%20Reference)))

(event EventTick
  (params (DeltaSeconds :type Float%20%28single-precision%29)))

(event EventActorLoaded
  (bind _returnvalue (Pawn|GetController))
  (bind _currentlyappliedeffects (Variables|Default|GetCurrentlyAppliedEffects))
  (if (Variables|Default|GetbDead)
    ;[0 0.5057 1] Because of how SaveSystem is designed it's much easier to fake the destruction, by simply "disabling" the actor
    (Rendering|SetActorHiddenInGame true)
    (Actor|Tick|SetActorTickEnabled false)
    (Collision|SetActorEnableCollision false)
    (Utilities|IsValid _returnvalue
      (:Is%20Valid
        (AI|Navigation|StopMovement _returnvalue)
        (Pawn|UnPossess _returnvalue))
      (:Is%20Not%20Valid
        _))
    (Variables|/Script/Engine.CharacterMovementComponent|SetMaxWalkSpeed (Variables|Character|GetCharacterMovement) 0.0)
    (Variables|Default|SetFinishedDeathAnim true)
    ;[0.1896 1 0] Clear Effects
    (for _array_element _currentlyappliedeffects
      (Actor|DestroyActor _array_element))
    (Utilities|Array|Clear _currentlyappliedeffects)))

(event EventDie
  (bind _returnvalue (Pawn|GetController))
  (bind _currentlyappliedeffects (Variables|Default|GetCurrentlyAppliedEffects))
  (|CallParentFunction)
  (if (not (Variables|Default|GetFinishedDeathAnim))
    (Audio|PlaySound2D 0 1.0 1.0 0.0 0 0)
    (Utilities|PlayAnimation "/Game/Assets/Sprites/BadGuy/temp/Die/PlaceHolderBadGuyDie1.PlaceHolderBadGuyDie1" false
      (:Success
        (Development|PrintString "playing anim"))
      (:Fail
        (Development|PrintString "no anim"))
      (:Completed
        ;[0 0.5057 1] Because of how SaveSystem is designed it's much easier to fake the destruction, by simply "disabling" the actor
        (Rendering|SetActorHiddenInGame true)
        (Actor|Tick|SetActorTickEnabled false)
        (Collision|SetActorEnableCollision false)
        (Utilities|IsValid _returnvalue
          (:Is%20Valid
            (AI|Navigation|StopMovement _returnvalue)
            (Pawn|UnPossess _returnvalue))
          (:Is%20Not%20Valid
            _))
        (Variables|/Script/Engine.CharacterMovementComponent|SetMaxWalkSpeed (Variables|Character|GetCharacterMovement) 0.0)
        (Variables|Default|SetFinishedDeathAnim true)
        ;[0.1896 1 0] Clear Effects
        (for _array_element _currentlyappliedeffects
          (Actor|DestroyActor _array_element))
        (Utilities|Array|Clear _currentlyappliedeffects)))))

(event EventInteract
  (params (Interactor :type Actor%20Object%20Reference))
  (bind _dialog (Variables|Default|GetDialog))
  ;[1 1 1] Start dialog
  (Utilities|Casting|CastToPlayerBase Interactor)
  (Utilities|IsValid _dialog
    (:Is%20Valid
      (bind _returnvalue (UserInterface|CreateWidget "/Game/Blueprints/UI/Dialog/UMG_Dialog.UMG_Dialog_C" 0 _dialog self))
      (UserInterface|Viewport|AddtoViewport _returnvalue 0))))

(fn ConstructionScript)

(fn DealDamage
  (params (Damage :type Integer) (DamageDealer :type Actor%20Object%20Reference) (SpecialEffect :type Special%20Effect%20Class%20Reference))
  (bind _returnvalue (|CallParentFunction Damage DamageDealer SpecialEffect))
  (Development|PrintString (Utilities|String|Append (Utilities|GetDisplayName self) " Received: " (Utilities|String|ToString(Integer) Damage) "dmg. From" (Utilities|GetDisplayName DamageDealer)) true true "(R=0.310241,G=1.000000,B=0.235314,A=1.000000)")
  (return _returnvalue))

(fn ComponentstoSave
  (return 0))
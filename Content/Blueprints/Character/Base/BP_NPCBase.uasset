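; Base NPC character Blueprint that handles controller fallback and death, including the experience reward display.
; On BeginPlay it spawns and possesses with a fallback controller class if it has none.
; Death plays a sound, animation and timeline-driven rising XP text.
; Afterwards the actor is hidden and disabled and its effects cleared, faking destruction to suit the SaveSystem; a custom event reapplies this state when Dead.
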(event Custom|CustomEvent
  (bind _returnvalue (Pawn|GetController))
  (bind _currentlyappliedeffects (Variables|Default|GetCurrentlyAppliedEffects))
  (if (Variables|Default|GetbDead)
    ;[0 0.5057 1] Because of how SaveSystem is designed it's much easier to fake the destruction, by simply "disabling" the actor
    (Rendering|SetActorHiddenInGame true)
    (Actor|Tick|SetActorTickEnabled false)
    (Collision|SetActorEnableCollision false)
    (Utilities|IsValid _returnvalue
      (:Is%20Valid
        (AI|Navigation|StopMovement _returnvalue)
        (Pawn|UnPossess _returnvalue))
      (:Is%20Not%20Valid
        _))
    (Variables|/Script/Engine.CharacterMovementComponent|SetMaxWalkSpeed (Variables|Character|GetCharacterMovement) 0.0)
    (Variables|Default|SetFinishedDeathAnim true)
    ;[0.1896 1 0] Clear Effects
    (for _array_element _currentlyappliedeffects
      (Actor|DestroyActor _array_element))
    (Utilities|Array|Clear _currentlyappliedeffects)))

(event EventBeginPlay
  ;[1 1 1] Begin play
  (CallFunction|SetupController)
  (|CallParentFunction)
  (Collision|IgnoreActorwhenMoving (Variables|Default|GetCollision) self true))

(event EventDie
  (bind _returnvalue (Pawn|GetController))
  (bind _returnvalue_2 (Pawn|GetController))
  (bind _currentlyappliedeffects (Variables|Default|GetCurrentlyAppliedEffects))
  (|CallParentFunction)
  (if (not (Variables|Default|GetFinishedDeathAnim))
    (Audio|Components|Audio|Play (Variables|Default|GetExpTimeline))
    (Rendering|SetVisibility (Variables|Default|GetExpTextRenderComponent) true false)
    (Rendering|Components|TextRender|SetText (Variables|Default|GetExpTextRenderComponent) (Utilities|Text|ToText(String) (Utilities|String|Append (Utilities|String|ToString(Integer) (Variables|Default|GetExperience)) "xp")))
    (Audio|PlaySound2D 0 1.0 1.0 0.0 0 0)
    (Utilities|PlayAnimation (Variables|Default|GetDeathAnimation) false
      (:Success
        (Utilities|IsValid _returnvalue
          (:Is%20Valid
            (Pawn|UnPossess _returnvalue))))
      (:Fail
        (Development|PrintString "no anim"))
      (:Completed
        ;[0 0.5057 1] Because of how SaveSystem is designed it's much easier to fake the destruction, by simply "disabling" the actor
        (Rendering|SetActorHiddenInGame true)
        (Actor|Tick|SetActorTickEnabled false)
        (Collision|SetActorEnableCollision false)
        (Utilities|IsValid _returnvalue_2
          (:Is%20Valid
            (AI|Navigation|StopMovement _returnvalue_2)
            (Pawn|UnPossess _returnvalue_2))
          (:Is%20Not%20Valid
            _))
        (Variables|/Script/Engine.CharacterMovementComponent|SetMaxWalkSpeed (Variables|Character|GetCharacterMovement) 0.0)
        (Variables|Default|SetFinishedDeathAnim true)
        ;[0.1896 1 0] Clear Effects
        (for _array_element _currentlyappliedeffects
          (Actor|DestroyActor _array_element))
        (Utilities|Array|Clear _currentlyappliedeffects)))))

(fn ConstructionScript)

(fn SetupController
  (bind _fallbackcontrollerclass (Variables|Default|GetFallbackControllerClass))
  (Utilities|IsValid (Pawn|GetController)
    (:Is%20Valid
      _)
    (:Is%20Not%20Valid
      (if (Utilities|IsValidClass _fallbackcontrollerclass)
        (bind _returnvalue (Game|SpawnActorfromClass _fallbackcontrollerclass (Transformation|GetActorTransform) "AlwaysSpawn" 0 0))
        (Pawn|Possess _returnvalue self)
        (Class|EnemyAIBase|Setup _returnvalue))))
  (return))
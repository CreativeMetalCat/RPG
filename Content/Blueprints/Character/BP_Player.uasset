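; BP_Player is the player Blueprint that owns the HUD and seeds the player's quest list.
; On BeginPlay it creates UMG_HUD, then passes every DT_Quests row to AddQuestToQuestArray, intended to leave completed quests intact.
; Update events refresh quest and player info on the HUD, and LevelUp plays a stinger sound.
; A development-only Tick rotates Arrow1 to show CurrentDirection.
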(event EventBeginPlay
  (|CallParentFunction)
  ;[0.1563 1 0.1972] Create HUD
  (bind _returnvalue (UserInterface|CreateWidget "/Game/Blueprints/UI/UMG_HUD.UMG_HUD_C" 0 self))
  (bind _output_get (Variables|Default|SetHUD _returnvalue))
  (UserInterface|Viewport|AddtoViewport _output_get 0)
  ;[0.3991 0.436 1] This adds every quest that player doesn't have
  (bind _outrownames (DataTable|GetDataTableRowNames "/Game/DataTables/DT_Quests.DT_Quests"))
  (for _array_element _outrownames
    (bind _returnvalue_2 (Utilities|GetDataTableRow "/Game/DataTables/DT_Quests.DT_Quests" _array_element)
      (:then
        (Class|RPGCharacter|AddQuesttoQuestArray _returnvalue_2) ; This way if player has quest completed it won't be overriden
      ))))

(event Collision|EventActorBeginOverlap
  (params (OtherActor :type Actor%20Object%20Reference)))

(event EventTick
  (params (DeltaSeconds :type Float%20%28single-precision%29))
  ;[1 0 0] DEVELOPMENT ONLY
  (Transformation|SetRelativeRotation (Variables|Default|GetArrow1) (Utilities|Select :Index (Variables|Default|GetCurrentDirection) :ED_Up "0,270.000000, 0" :ED_Down "0,90.000000, 0" :ED_Right "0, 0, 0" :ED_Left "0,180.000000, 0") false false))

(event EventUpdateQuestDisplayInfo
  (bind _hud (Variables|Default|GetHUD)
    (:then
      (Default|UpdateQuestInfo _hud))
    (:else)))

(event EventUpdatePlayerInfo
  (bind _hud (Variables|Default|GetHUD)
    (:then
      (Default|UpdatePlayerInfo _hud))
    (:else)))

(event EventLevelUp
  (Audio|PlaySound2D "/Game/Assets/Retro_8Bit_Sounds/Music/Wavs/retro__musical_stinger_02.retro__musical_stinger_02" 1.0 1.0 0.0 0 0))

(fn ConstructionScript)
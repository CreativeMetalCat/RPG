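; Test enemy character Blueprint that adds death feedback and damage logging on top of its parent class.
; Its Die event plays a 2D explosion sound and a placeholder death animation, printing whether the animation starts, then destroys the actor when it completes.
; The DealDamage override calls the parent implementation, prints the receiver, amount and dealer as debug text, and returns the parent's result.
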(event EventBeginPlay)

(event Collision|EventActorBeginOverlap
  (params (OtherActor :type Actor%20Object%20Reference)))

(event EventTick
  (params (DeltaSeconds :type Float%20%28single-precision%29)))

(event EventDie
  (Audio|PlaySound2D "/Game/Assets/Retro_8Bit_Sounds/Explosion/Wavs/retro_explosion_short_06.retro_explosion_short_06" 1.0 1.0 0.0 0 0)
  (Utilities|PlayAnimation "/Game/Assets/Sprites/BadGuy/temp/Die/PlaceHolderBadGuyDie1.PlaceHolderBadGuyDie1"
    (:Success
      (Development|PrintString "playing anim"))
    (:Fail
      (Development|PrintString "no anim"))
    (:Completed
      (Actor|DestroyActor))))

(fn ConstructionScript)

(fn DealDamage
  (params (Damage :type Integer) (DamageDealer :type Actor%20Object%20Reference) (SpecialEffect :type Special%20Effect%20Class%20Reference))
  (bind _returnvalue (|CallParentFunction Damage 0 SpecialEffect))
  (Development|PrintString (Utilities|String|Append (Utilities|GetDisplayName self) " Received: " (Utilities|String|ToString(Integer) Damage) "dmg. From" (Utilities|GetDisplayName DamageDealer)) true true "(R=0.310241,G=1.000000,B=0.235314,A=1.000000)")
  (return _returnvalue))
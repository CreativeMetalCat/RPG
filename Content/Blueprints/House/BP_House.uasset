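; BP_House is an interactable 2D house whose flipbook door teleports whoever uses it indoors.
; Interact, when not Locked, caches the interactor and plays the non-looping opening flipbook once.
; When that flipbook finishes, the cached interactor moves to InDoorsLocationActor's location and the opening flag clears.
; PlayClosingAnim is a separate event for the closing flipbook, and DealDamage is a stub returning zero.
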(event OnFinishedPlaying(FB_Small_House_Idle_Front)
  (bind _indoorslocationactor (Variables|InDoors|GetInDoorsLocationActor))
  (bind _interactorcached (Variables|Default|GetInteractorCached))
  ;[1 1 1] On animation end
  (if (Variables|Default|GetOpening)
    (Utilities|IsValid _indoorslocationactor
      (:Is%20Valid
        (Utilities|IsValid _interactorcached
          (:Is%20Valid
            (Transformation|SetActorLocation _interactorcached (Transformation|GetActorLocation _indoorslocationactor) false false)
            (Variables|Default|SetOpening false)))))))

(event Custom|PlayClosingAnim
  (bind _fb_small_house_idle_front (Variables|Default|GetFB_Small_House_Idle_Front))
  ;[1 1 1] Play closing anim
  (Sprite|SetFlipbook _fb_small_house_idle_front (Variables|Anim|GetClosingAnim))
  (Audio|Components|Audio|Play _fb_small_house_idle_front))

(event EventBeginPlay)

(event Collision|EventActorBeginOverlap
  (params (OtherActor :type Actor%20Object%20Reference)))

(event EventTick
  (params (DeltaSeconds :type Float%20%28single-precision%29)))

(event EventInteract
  (params (Interactor :type Actor%20Object%20Reference))
  (bind _fb_small_house_idle_front (Variables|Default|GetFB_Small_House_Idle_Front))
  (if (not (Variables|Default|GetLocked))
    (Variables|Default|SetInteractorCached Interactor)
    (if (not (Variables|Default|GetOpening))
      (Sprite|SetFlipbook _fb_small_house_idle_front (Variables|Anim|GetOpeningAnim))
      (Audio|Components|Audio|Play _fb_small_house_idle_front)
      (Variables|Default|SetOpening true))))

(fn ConstructionScript
  (Components|Timeline|SetLooping (Variables|Default|GetFB_Small_House_Idle_Front) false))

(fn DealDamage
  (params (Damage :type Integer) (DamageDealer :type Actor%20Object%20Reference) (SpecialEffect :type Special%20Effect%20Class%20Reference))
  (return 0))
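; BP_LightRay is a projectile that deals damage to the first actor it overlaps other than its owning character, then destroys itself.
; On BeginPlay it passes its max speed and initial velocity to a 2D projectile movement component and initializes it.
; The collision component ignores the owner while moving to avoid self-damage.
; Damage is sent as a DealDamageMessage carrying the dealer and a special effect.
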(event OnComponentBeginOverlap(CollisionComponent)
  (params (OverlappedComponent :type Primitive%20Component%20Object%20Reference) (OtherActor :type Actor%20Object%20Reference) (OtherComp :type Primitive%20Component%20Object%20Reference) (OtherBodyIndex :type Integer) (bFromSweep :type Boolean) (SweepResult :type Hit%20Result%20Structure%20%28by%20ref%29))
  ;[1 1 1] On hit
  (if (!= (Variables|Default|GetOwningCharacter) OtherActor)
    (Class|Interaction|DealDamage(Message) OtherActor (Variables|Default|GetDamage) (Variables|Default|GetOwningCharacter) (Variables|Default|GetSpecial%20Effect))
    (Actor|DestroyActor)))

(event EventBeginPlay
  (bind _bp_projectile2dmovement (Variables|Default|GetBP_Projectile2dMovement))
  ;[1 1 1] Begin Play
  (Variables|/Script/RPGCore.Projectile2dMovementComponent|SetMaxSpeed _bp_projectile2dmovement (Variables|Default|GetMax%20Speed))
  (Class|Projectile2dMovementComponent|SetNewInitialVelocity _bp_projectile2dmovement (Variables|Default|GetInitial%20Velocity))
  (Class|Projectile2dMovementComponent|Init _bp_projectile2dmovement)
  ;[1 1 1] Ignore player when moving to avoid self damaging
  (Collision|IgnoreActorwhenMoving (Variables|Default|GetCollisionComponent) (Variables|Default|GetOwningCharacter) true))

(fn ConstructionScript)
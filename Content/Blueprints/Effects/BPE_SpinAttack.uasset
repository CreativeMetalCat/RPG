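; Spin attack effect actor that performs a radial melee hit when an RPG character applies it.
; ApplyEffect checks the creator for an equipped weapon, plays the spin flipbook, then sphere-overlaps Pawns around the origin, excluding the creator.
; Each hit receives weapon attack times the creator's attack power through a damage message.
; The effect destroys itself only on the weapon path, and its Radius variable is unused in favor of a hardcoded radius.
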(event EventBeginPlay)

(event EventTick
  (params (DeltaSeconds :type Float%20%28single-precision%29)))

(event EventApplyEffect
  (params (CreatorOfEffect :type Actor%20Object%20Reference) (Origin :type Vector :default "0, 0, 0") (WorldContext :type World%20Object%20Reference) (TargetActor :type Actor%20Object%20Reference))
  (|CallParentFunction CreatorOfEffect Origin WorldContext TargetActor)
  (bind _asrpgcharacter_base (Utilities|Casting|CastToRPGCharacterBase CreatorOfEffect))
  (if (.has (Class|RPGCharacterBase|GetCurrentItemforType _asrpgcharacter_base "EIT_Weapon"))
    (Class|RPGCharacterBase|PlayFlipbookAnimation _asrpgcharacter_base "/Game/Assets/Sprites/Character/SpinAttack/FB_Player_Spin_Attack.FB_Player_Spin_Attack" false)
    (bind (_outactors _returnvalue) (Collision|SphereOverlapActors Origin 2e+02 (Utilities|Array|MakeArray "ObjectTypeQuery3") "/Script/Engine.Actor" (Utilities|Array|MakeArray CreatorOfEffect)))
    (if _returnvalue
      (for _array_element _outactors
        (Class|Interaction|DealDamage(Message) _array_element (* (.Attack (Utilities|Struct|BreakItemInfo (.ReturnValue (Class|RPGCharacterBase|GetCurrentItemforType _asrpgcharacter_base "EIT_Weapon")))) (Variables|/Script/RPGCore.RPGCharacterBase|GetAttackPower _asrpgcharacter_base)) CreatorOfEffect 0)))
    (Actor|DestroyActor)))

(fn ConstructionScript)
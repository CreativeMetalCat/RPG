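; BP_DamageSphere is a charge attack effect actor that damages actors overlapping its sphere.
; On BeginPlay it sizes the Sphere component from its Radius variable.
; When another actor begins overlapping the sphere, it sends that actor a DealDamage message with Damage, Damager and SpecialEffect, skipping the Damager itself.
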(event OnComponentBeginOverlap(Sphere)
  (params (OverlappedComponent :type Primitive%20Component%20Object%20Reference) (OtherActor :type Actor%20Object%20Reference) (OtherComp :type Primitive%20Component%20Object%20Reference) (OtherBodyIndex :type Integer) (bFromSweep :type Boolean) (SweepResult :type Hit%20Result%20Structure%20%28by%20ref%29))
  ;[1 1 1] Damage
  (if (!= OtherActor (Variables|Default|GetDamager))
    (Class|Interaction|DealDamage(Message) OtherActor (Variables|Default|GetDamage) (Variables|Default|GetDamager) (Variables|Default|GetSpecial%20Effect))))

(event EventBeginPlay
  ;[1 1 1] Setup
  (Components|Sphere|SetSphereRadius (Variables|Default|GetSphere) (Variables|Default|GetRadius) true))

(event Collision|EventActorBeginOverlap
  (params (OtherActor :type Actor%20Object%20Reference)))

(event EventTick
  (params (DeltaSeconds :type Float%20%28single-precision%29)))

(fn ConstructionScript)
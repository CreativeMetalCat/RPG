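; Fire ring effect that deals area damage around an origin point when applied, extending a parent effect's ApplyEffect.
; It spawns a scaled-up fire ring flipbook at the origin, then sphere-overlaps pawns within Radius, excluding the effect's creator.
; Each hit actor receives BaseDamage through DealDamageMessage with BPE_Fire as the special effect, and the effect actor then destroys itself.
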(event EventBeginPlay)

(event EventTick
  (params (DeltaSeconds :type Float%20%28single-precision%29)))

(event EventApplyEffect
  (params (CreatorOfEffect :type Actor%20Object%20Reference) (Origin :type Vector :default "0, 0, 0") (WorldContext :type World%20Object%20Reference) (TargetActor :type Actor%20Object%20Reference))
  (|CallParentFunction CreatorOfEffect Origin WorldContext TargetActor)
  (Game|SpawnActorfromClass "/Game/Blueprints/FlipbookAnimation/BP_FlipbookEffect.BP_FlipbookEffect_C" (Math|Transform|MakeTransform Origin "0, 0, 0" "4.000000,4.000000,4.000000") "AlwaysSpawn" 0 "/Game/Assets/Sprites/Abilities/Firering/FB_Ability_firering1.FB_Ability_firering1" false 0)
  (bind (_outactors _returnvalue) (Collision|SphereOverlapActors Origin (Variables|Default|GetRadius) (Utilities|Array|MakeArray "ObjectTypeQuery3") "/Script/Engine.Actor" (Utilities|Array|MakeArray CreatorOfEffect)))
  (if _returnvalue
    (for _array_element _outactors
      (Class|Interaction|DealDamage(Message) _array_element (Variables|Default|GetBaseDamage) CreatorOfEffect "/Game/Blueprints/Effects/BPE_Fire.BPE_Fire_C")))
  (Actor|DestroyActor))

(fn ConstructionScript)
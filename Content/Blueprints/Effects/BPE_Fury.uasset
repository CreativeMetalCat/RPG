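; BPE_Fury is a Fury effect Blueprint that modifies an RPG character's attack power.
; On apply, it casts the effect's creator to RPGCharacterBase, adds Increase to AttackPower and plays a Fury flipbook matching the character's facing direction.
; When the effect ends, it adds Increase to the creator's AttackPower again rather than subtracting it, then calls the parent end logic.
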(event EventBeginPlay)

(event EventTick
  (params (DeltaSeconds :type Float%20%28single-precision%29)))

(event EventApplyEffect
  (params (CreatorOfEffect :type Actor%20Object%20Reference) (Origin :type Vector :default "0, 0, 0") (WorldContext :type World%20Object%20Reference) (TargetActor :type Actor%20Object%20Reference))
  (bind _asrpgcharacter_base (Utilities|Casting|CastToRPGCharacterBase CreatorOfEffect))
  (Variables|/Script/RPGCore.RPGCharacterBase|SetAttackPower _asrpgcharacter_base (+ (Variables|/Script/RPGCore.RPGCharacterBase|GetAttackPower _asrpgcharacter_base) (Variables|Default|GetIncrease)))
  (Class|RPGCharacterBase|PlayFlipbookAnimation _asrpgcharacter_base (Utilities|Select :Index (Variables|/Script/RPGCore.RPGCharacterBase|GetCurrentDirection _asrpgcharacter_base) :ED_Up "/Game/Assets/Sprites/Character/Fury/Up/FB_Player_Fury_Up1.FB_Player_Fury_Up1" :ED_Down "/Game/Assets/Sprites/Character/Fury/Down/FB_Player_Fury_Down1.FB_Player_Fury_Down1" :ED_Right "/Game/Assets/Sprites/Character/Fury/Right/FB_PLayer_Fury_Right1.FB_PLayer_Fury_Right1" :ED_Left "/Game/Assets/Sprites/Character/Fury/Left/FB_Player_Fury_Leftt1.FB_Player_Fury_Leftt1") false))

(event EventOnEffectEnds
  (bind _asrpgcharacter_base (Utilities|Casting|CastToRPGCharacterBase (Variables|Default|GetCreator))
    (:then
      (Variables|/Script/RPGCore.RPGCharacterBase|SetAttackPower _asrpgcharacter_base (+ (Variables|/Script/RPGCore.RPGCharacterBase|GetAttackPower _asrpgcharacter_base) (Variables|Default|GetIncrease))))
    (:CastFailed
      _))
  (|CallParentFunction))

(fn ConstructionScript)
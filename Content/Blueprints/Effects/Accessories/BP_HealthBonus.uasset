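; BP_HealthBonus is an accessory effect that raises the wearing RPG character's MaxHealth.
; Putting it on calls the parent handler and multiplies the owner's MaxHealth by 1.3, while taking it off scales the Creator's by 0.76, an approximate inverse.
; Tick also reapplies the 1.3 multiplier to the Creator on every call, so the increase compounds; all results are truncated to integers.
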(event EventBeginPlay)

(event EventTick
  (params (DeltaSeconds :type Float%20%28single-precision%29))
  (bind _asrpgcharacter_base (Utilities|Casting|CastToRPGCharacterBase (Variables|Default|GetCreator)))
  (Variables|/Script/RPGCore.RPGCharacterBase|SetMaxHealth _asrpgcharacter_base (Math|Float|Truncate (* (Variables|/Script/RPGCore.RPGCharacterBase|GetMaxHealth _asrpgcharacter_base) 1.3))))

(event EventOnAccessoryPuton
  (params (accessoryOwner :type Actor%20Object%20Reference))
  (|CallParentFunction accessoryOwner)
  (bind _asrpgcharacter_base (Utilities|Casting|CastToRPGCharacterBase accessoryOwner))
  (Variables|/Script/RPGCore.RPGCharacterBase|SetMaxHealth _asrpgcharacter_base (Math|Float|Truncate (* (Variables|/Script/RPGCore.RPGCharacterBase|GetMaxHealth _asrpgcharacter_base) 1.3)))
  (Development|PrintString "Started"))

(event EventOnAccessoryTakeoff
  (bind _asrpgcharacter_base (Utilities|Casting|CastToRPGCharacterBase (Variables|Default|GetCreator)))
  (Variables|/Script/RPGCore.RPGCharacterBase|SetMaxHealth _asrpgcharacter_base (Math|Float|Truncate (* (Variables|/Script/RPGCore.RPGCharacterBase|GetMaxHealth _asrpgcharacter_base) 0.76)))
  (Development|PrintString "Eneed"))

(fn ConstructionScript)
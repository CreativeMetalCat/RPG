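; Charge attack ability effect that roots the RPG character while the button is held, then dashes on release.
; On apply, it zeroes walk speed and binds the creator's button-release message.
; Release restores speed, disables input, plays a directional hit flipbook and attaches a spawned damage sphere.
; Tick feeds movement along the facing direction until a timer restores input, destroys the sphere and ends the effect.
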(event Custom|StopARunning
  ;[1 1 1] Stop running
  (Variables|Default|SetDoInput false)
  (Input|EnableInput (Variables|Default|GetStoredPlayerInfo) (Game|GetPlayerController 0))
  (Actor|DestroyActor (Variables|Default|GetDamagingSphere))
  (Class|SpecialEffect|OnEffectEnds))

(event EventTick
  (params (DeltaSeconds :type Float%20%28single-precision%29))
  (bind _storedplayerinfo (Variables|Default|GetStoredPlayerInfo))
  ;[1 1 1] Add movement input
  (if (Variables|Default|GetDoInput)
    (Utilities|IsValid _storedplayerinfo
      (:Is%20Valid
        (Pawn|Input|AddMovementInput (Variables|Default|GetStoredPlayerInfo) (Utilities|Select :Index (Variables|/Script/RPGCore.RPGCharacterBase|GetCurrentDirection _storedplayerinfo) :ED_Up "0,-1.000000, 0" :ED_Down "0,1.000000, 0" :ED_Right "1.000000, 0, 0" :ED_Left "-1.000000, 0, 0") 1.0 false)))))

(event EventOnAbilityButtonReleased
  (bind _creator (Variables|Default|GetCreator))
  ;[1 1 1] On button released
  (bind _asrpgcharacter_base (Utilities|Casting|CastToRPGCharacterBase (Variables|Default|GetCreator)))
  (bind _output_get (Variables|Default|SetStoredPlayerInfo _asrpgcharacter_base))
  (Variables|/Script/Engine.CharacterMovementComponent|SetMaxWalkSpeed (Variables|/Script/Engine.Character|GetCharacterMovement _output_get) (Variables|/Script/RPGCore.RPGCharacterBase|GetDefaultMovementSpeed _output_get))
  (Input|DisableInput _output_get (Game|GetPlayerController 0))
  (Class|RPGCharacterBase|PlayFlipbookAnimation _output_get (Utilities|Select :Index (Variables|/Script/RPGCore.RPGCharacterBase|GetCurrentDirection _output_get) :ED_Up "/Game/Assets/Sprites/Character/ChargeAttack/Up/FB_Player_Charge_Hit_Up1.FB_Player_Charge_Hit_Up1" :ED_Down "/Game/Assets/Sprites/Character/ChargeAttack/Down/FB_Player_Charge_Hit_Down1.FB_Player_Charge_Hit_Down1" :ED_Right "/Game/Assets/Sprites/Character/ChargeAttack/Left/FB_Charge_Hit_Side1.FB_Charge_Hit_Side1" :ED_Left "/Game/Assets/Sprites/Character/ChargeAttack/Right/FB_PlayerCharge_Hit_Side_Right1.FB_PlayerCharge_Hit_Side_Right1") true)
  (Development|PrintString "Dash")
  (Variables|Default|SetDoInput true)
  (Utilities|Time|SetTimerbyEvent (delegate Custom|StopARunning) (Variables|Default|GetRunningTime))
  ;[1 1 1] Spawn and attach sphere
  (bind _returnvalue (Game|SpawnActorfromClass "/Game/Blueprints/Effects/ChargeAttack/BP_DamageSphere.BP_DamageSphere_C" (Transformation|GetActorTransform _creator) "AlwaysSpawn" 0 (Math|Float|Truncate (Variables|Default|GetDamage)) _creator 0 6e+01 0))
  (Transformation|AttachActorToActor _returnvalue _creator "None" "SnapToTarget" "SnapToTarget" "SnapToTarget" true)
  (Variables|Default|SetDamagingSphere _returnvalue))

(event EventApplyEffect
  (params (CreatorOfEffect :type Actor%20Object%20Reference) (Origin :type Vector :default "0, 0, 0") (WorldContext :type World%20Object%20Reference) (TargetActor :type Actor%20Object%20Reference))
  ;[1 1 1] On Summon
  (|CallParentFunction CreatorOfEffect Origin WorldContext TargetActor)
  (Class|Interaction|BindEventonAbilityButtonReleased(Message) CreatorOfEffect self)
  (bind _asrpgcharacter_base (Utilities|Casting|CastToRPGCharacterBase CreatorOfEffect)
    (:then
      (Variables|/Script/Engine.CharacterMovementComponent|SetMaxWalkSpeed (Variables|/Script/Engine.Character|GetCharacterMovement _asrpgcharacter_base) 0.0)
      (Development|PrintString "Start waiting Dash" false false))
    (:CastFailed
      (Development|PrintString "Ho" false false))))

(fn ConstructionScript)
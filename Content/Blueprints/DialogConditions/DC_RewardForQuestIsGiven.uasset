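; Dialog condition that checks whether the considering player has already been given the reward for a configured quest.
; It resolves the Quest row handle to a DevName, looks that quest up on the controlled BP_Player and reads its Rewarded flag.
; A failed cast, missing row or quest the player lacks counts as not rewarded, and InverseAnswer flips every result.
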(fn IsConditionMet
  (params (ConsideringPlayer :type Player%20Controller%20Object%20Reference) (NPCActor :type Actor%20Object%20Reference))
  (bind _quest (Variables|Default|GetQuest))
  (bind (_datatable _rowname) (Utilities|Struct|BreakDataTableRowHandle _quest))
  (bind _asbp_player (Utilities|Casting|CastToBP_Player (Pawn|GetControlledPawn ConsideringPlayer))
    (:then
      (bind _returnvalue (Utilities|GetDataTableRow _datatable _rowname)
        (:then
          (if (.hasQuest (Class|PlayerBase|GetQuestInfo _asbp_player (.DevName (Utilities|Struct|BreakQuestInfo _returnvalue))))
            (return (select (Variables|Default|GetInverseAnswer) (not (Utilities|Struct|BreakQuestInfo (.ReturnValue (Class|PlayerBase|GetQuestInfo _asbp_player (.DevName (Utilities|Struct|BreakQuestInfo _returnvalue)))))) (Utilities|Struct|BreakQuestInfo (.ReturnValue (Class|PlayerBase|GetQuestInfo _asbp_player (.DevName (Utilities|Struct|BreakQuestInfo _returnvalue)))))))
            (else
              _)))
        (:RowNotFound
          _)))
    (:CastFailed
      _))
  (return (select (Variables|Default|GetInverseAnswer) true false)))
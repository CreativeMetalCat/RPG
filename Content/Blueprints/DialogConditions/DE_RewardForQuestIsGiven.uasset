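; Dialog condition that checks whether the considering player has already been given the reward for a specified quest.
; It looks up the quest row in DT_Quests, then queries the controlled BP_Player's quest info by DevName for its Rewarded flag.
; A failed cast, missing row or absent quest counts as not rewarded, and InverseAnswer flips the result in every case.
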(fn IsConditionMet
  (params (ConsideringPlayer :type Player%20Controller%20Object%20Reference) (NPCActor :type Actor%20Object%20Reference))
  (bind _asbp_player (Utilities|Casting|CastToBP_Player (Pawn|GetControlledPawn ConsideringPlayer))
    (:then
      (bind _returnvalue (Utilities|GetDataTableRow "/Game/DataTables/DT_Quests.DT_Quests" (.RowName (Utilities|Struct|BreakDataTableRowHandle (Variables|Default|GetQuest))))
        (:then
          (if (.hasQuest (Class|RPGCharacter|GetQuestInfo _asbp_player (.DevName (Utilities|Struct|BreakQuest _returnvalue))))
            (return (select (Variables|Default|GetInverseAnswer) (not (Utilities|Struct|BreakQuest (.ReturnValue (Class|RPGCharacter|GetQuestInfo _asbp_player (.DevName (Utilities|Struct|BreakQuest _returnvalue)))))) (Utilities|Struct|BreakQuest (.ReturnValue (Class|RPGCharacter|GetQuestInfo _asbp_player (.DevName (Utilities|Struct|BreakQuest _returnvalue)))))))
            (else
              _)))
        (:RowNotFound
          _)))
    (:CastFailed
      _))
  (return (select (Variables|Default|GetInverseAnswer) true false)))
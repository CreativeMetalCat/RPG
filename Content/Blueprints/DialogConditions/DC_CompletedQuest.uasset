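; Dialog condition that checks whether the considering player has completed a specified quest.
; It looks up the quest's row in DT_Quest and uses its DevName to query the BP_Player pawn's quest info for the Completed flag.
; InverseAnswer flips the result, and a failed cast, missing row or quest the player lacks counts as not completed.
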(fn IsConditionMet
  (params (ConsideringPlayer :type Player%20Controller%20Object%20Reference) (NPCActor :type Actor%20Object%20Reference))
  (bind _asbp_player (Utilities|Casting|CastToBP_Player (Pawn|GetControlledPawn ConsideringPlayer))
    (:then
      (bind _returnvalue (Utilities|GetDataTableRow "/Game/DataTables/DT_Quest.DT_Quest" (.RowName (Utilities|Struct|BreakDataTableRowHandle (Variables|Default|GetQuest))))
        (:then
          (if (.hasQuest (Class|RPGCharacterBase|GetQuestInfo _asbp_player (.DevName (Utilities|Struct|BreakQuestInfo _returnvalue))))
            (return (select (Variables|Default|GetInverseAnswer) (not (Utilities|Struct|BreakQuestInfo (.ReturnValue (Class|RPGCharacterBase|GetQuestInfo _asbp_player (.DevName (Utilities|Struct|BreakQuestInfo _returnvalue)))))) (Utilities|Struct|BreakQuestInfo (.ReturnValue (Class|RPGCharacterBase|GetQuestInfo _asbp_player (.DevName (Utilities|Struct|BreakQuestInfo _returnvalue)))))))
            (else
              _)))
        (:RowNotFound
          _)))
    (:CastFailed
      _))
  (return (select (Variables|Default|GetInverseAnswer) true false)))
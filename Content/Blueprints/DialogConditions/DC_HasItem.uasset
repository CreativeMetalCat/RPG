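; DC_HasItem is a dialog condition that checks whether the player carries at least a required amount of an item.
; It resolves the item's DevName from a data table row handle named Quest, then looks that item up on the considering player's BP_Player pawn.
; InverseAnswer flips the result, including the failure cases of a wrong pawn, missing row or absent item.
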(fn IsConditionMet
  (params (ConsideringPlayer :type Player%20Controller%20Object%20Reference) (NPCActor :type Actor%20Object%20Reference))
  (bind _quest (Variables|Default|GetQuest))
  (bind (_datatable _rowname) (Utilities|Struct|BreakDataTableRowHandle _quest))
  (bind _asbp_player (Utilities|Casting|CastToBP_Player (Pawn|GetControlledPawn ConsideringPlayer))
    (:then
      (bind _returnvalue (Utilities|GetDataTableRow _datatable _rowname)
        (:then
          (if (.hasItem (Class|RPGCharacterBase|GetItembyName _asbp_player (.DevName (Utilities|Struct|BreakItemInfo _returnvalue))))
            (return (select (Variables|Default|GetInverseAnswer) (not (>= (Utilities|Struct|BreakItemInfo (.ReturnValue (Class|RPGCharacterBase|GetItembyName _asbp_player (.DevName (Utilities|Struct|BreakItemInfo _returnvalue))))) (Variables|Default|GetItemAmount))) (>= (Utilities|Struct|BreakItemInfo (.ReturnValue (Class|RPGCharacterBase|GetItembyName _asbp_player (.DevName (Utilities|Struct|BreakItemInfo _returnvalue))))) (Variables|Default|GetItemAmount))))
            (else
              _)))
        (:RowNotFound
          _)))
    (:CastFailed
      _))
  (return (select (Variables|Default|GetInverseAnswer) true false)))